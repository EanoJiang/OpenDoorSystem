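; Base demo prop Blueprint that drives an assigned skeletal mesh actor in the animation pack demo.
; On BeginPlay it sets the configured anim class on that actor and binds the Demo_AnimBP reset and begin events to its own Reset_Animation and Start_Animation events.
; Both events are empty hooks for children to override, and a missing actor prints a red on-screen error.
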(event `self.ReceiveBeginPlay`
  (bind _actor (`self.Actor`))
  (bind _skeletalmeshcomponent (`SkeletalMeshActor.SkeletalMeshComponent` _actor))
  ;[1 1 1] Giving the actor the proper animation blueprint.
  (`/Engine/EditorBlueprintResources/StandardMacros.IsValid` _actor
    (:`Is Valid`
      (`SkeletalMeshComponent.SetAnimInstanceClass` _skeletalmeshcomponent (`self.animation_blueprint_class`))
      ;[1 1 1] Linking skeletal events to blueprint events.
      (bind _asdemo_anim_bp (cast `/Game/OpenDoor/OpenAndCloseAnimationsPack/Demo_Assets/Demo_AnimBP` (`SkeletalMeshComponent.GetAnimInstance` _skeletalmeshcomponent)))
      (add `/Game/OpenDoor/OpenAndCloseAnimationsPack/Demo_Assets/Demo_AnimBP.Reset` _asdemo_anim_bp (delegate `Reset_Animation`))
      (add `/Game/OpenDoor/OpenAndCloseAnimationsPack/Demo_Assets/Demo_AnimBP.Begin` _asdemo_anim_bp (delegate `Start_Animation`)))
    (:`Is Not Valid`
      (`KismetSystemLibrary.PrintString` (`KismetStringLibrary.Concat_StrStr` (`KismetSystemLibrary.GetDisplayName` self) ": No valid skeletal mesh actor assigned.") true true (struct :`R` 1.0 :`A` 1.0) 10.0))))

(event `Reset_Animation`
  ;[1 1 1] Override in children to animate appropraitely
)

(event `Start_Animation`
  ;[1 1 1] Override in children to animate appropraitely
)

(fn `UserConstructionScript`)