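; Demo hinged box for the open and close animations pack, with a lid that animates open or closed.
; A timeline scales LidRotation into the relative roll of LidRoot, with its play rate set from PlayRate at BeginPlay.
; StartAnimation plays the timeline forward or in reverse according to PlayForward, and a separate ResetAnimation event resets the timeline's time.
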(event `self.ReceiveBeginPlay`
  (`parent.ReceiveBeginPlay`)
  ;[1 1 1] Set play rate
  (`TimelineComponent.SetPlayRate` (`self.animation_timeline`) (`self.play_rate`)))

(event `self.Start_Animation`
  ;[1 1 1] Start the animation based on whether or not forward playback is set
  (if (`self.play_forward?`)
    ;[1 1 1] Animate lid of the box
    (bind (_direction _float) (`Timeline|animation_timeline` :`NewTime` (`KismetMathLibrary.SelectFloat` 0.0 (`TimelineComponent.GetTimelineLength` (`self.animation_timeline`)) (`self.play_forward?`)) :!label _label)
      (:`Update`
        (`SceneComponent.K2_SetRelativeRotation` (`self.Lid_Root`) (`KismetMathLibrary.MakeRotator` (* (`self.lid_rotation`) _float)) false false)))
    (else
      (goto _label :!via `Reverse`))))

(event `self.Reset_Animation`
  ;[1 1 1] Reset the animation based on whether or not forward play back is set (0 for forward, 1 for reverse).
  (goto _label :!via `SetNewTime`))

(fn `UserConstructionScript`
  (`parent.UserConstructionScript`))