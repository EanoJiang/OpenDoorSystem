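; Demo window actor for an open/close animation pack that slides its Window component along local Z.
; BeginPlay applies PlayRate to the timeline, and StartAnimation plays it forward or in reverse according to PlayForward.
; The timeline's float track scales WindowDisplacement to set the window's relative height.
; A separate ResetAnimation event sets the timeline's time for replaying.
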(event `self.ReceiveBeginPlay`
  (`parent.ReceiveBeginPlay`)
  ;[1 1 1] Set play rate
  (`TimelineComponent.SetPlayRate` (`self.animation_timeline`) (`self.play_rate`)))

(event `self.Start_Animation`
  ;[1 1 1] Start the animation based on whether or not forward playback is set
  (if (`self.play_forward?`)
    ;[1 1 1] Animate window
    (bind (_direction _float) (`Timeline|animation_timeline` :`NewTime` (`KismetMathLibrary.SelectFloat` 0.0 (`TimelineComponent.GetTimelineLength` (`self.animation_timeline`)) (`self.play_forward?`)) :!label _label)
      (:`Update`
        (`SceneComponent.K2_SetRelativeLocation` (`self.window`) (`KismetMathLibrary.MakeVector` 0.0 0.0 (* (`self.window_displacement`) _float)) false false)))
    (else
      (goto _label :!via `Reverse`))))

(event `self.Reset_Animation`
  ;[1 1 1] Reset the animation based on whether or not forward play back is set (0 for forward, 1 for reverse).
  (goto _label :!via `SetNewTime`))

(fn `UserConstructionScript`
  (`parent.UserConstructionScript`))